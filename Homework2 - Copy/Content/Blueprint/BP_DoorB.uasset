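; BP_DoorB is a two-panel vertical sliding door that unlocks once the player has stepped on three separate trigger nodes.
; Each node's first overlap swaps its step and light materials and increments a counter.
; Tick polls the counter, then a timeline slides the panels apart and sets IsOpen.
; A second trigger warns about inactive nodes, and leaving DoorInteraction reverses the timeline, though IsOpen stays true.
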(event `self.ReceiveTick`
  (params (DeltaSeconds :type "Float (single-precision)"))
  ;[1 1 1] In the Door Range
  (if (`self.isOpen`)
    _
    (elif (>= (`self.Count`) 3.0)
      ;;[1 1 1] Do The Action If all the conditions are true
      (bind (_direction _newtrack_0) (`Timeline|Timeline_0` :!via `PlayFromStart` :!label _label)
        (:`Update`
          (`SceneComponent.K2_SetRelativeLocation` (`self.DoorUp`) (`KismetMathLibrary.VLerp` (`self.StartingPointDoorUp`) (`KismetMathLibrary.MakeVector` (.x (`self.StartingPointDoorUp`)) (.y (`self.StartingPointDoorUp`)) 333.583008) _newtrack_0) false false)
          (`SceneComponent.K2_SetRelativeLocation` (`self.DoorDown`) (`KismetMathLibrary.VLerp` (`self.StartingPointDoorDown`) (`KismetMathLibrary.MakeVector` (.x (`self.StartingPointDoorDown`)) (.y (`self.StartingPointDoorDown`)) -205.75) _newtrack_0) false false)
          (set `self.isOpen` true))))))

(event `self.ReceiveBeginPlay`
  ;[1 1 1] Start
  (set `self.StartingPointDoorUp` (`SceneComponent.RelativeLocation` (`self.DoorUp`)))
  (set `self.StartingPointDoorDown` (`SceneComponent.RelativeLocation` (`self.DoorDown`)))
  (`PrimitiveComponent.SetMaterial` (`self.Step 1`) 0 "/Game/Blueprint/M_Close.M_Close")
  (`PrimitiveComponent.SetMaterial` (`self.Step 2`) 0 "/Game/Blueprint/M_Close.M_Close")
  (`PrimitiveComponent.SetMaterial` (`self.Light 2`) 0 "/Game/Blueprint/M_Close.M_Close")
  (`PrimitiveComponent.SetMaterial` (`self.Light 1`) 0 "/Game/Blueprint/M_Close.M_Close")
  (`PrimitiveComponent.SetMaterial` (`self.Light 3`) 0 "/Game/Blueprint/M_Close.M_Close")
  (`PrimitiveComponent.SetMaterial` (`self.Step 3`) 0 "/Game/Blueprint/M_Close.M_Close")
  (set `self.Check 1` false)
  (set `self.Check 2` false)
  (set `self.Check 3` false)
  (set `self.isOpen` false)
  (set `self.Count` 0.0))

(event `self.DoorInteraction2.OnComponentBeginOverlap`
  (params (OverlappedComponent :type "PrimitiveComponent Object Reference") (OtherActor :type "Actor Object Reference") (OtherComp :type "PrimitiveComponent Object Reference") (OtherBodyIndex :type Integer) (bFromSweep :type Boolean) (SweepResult :type "HitResult Structure (by ref)"))
  ;[1 1 1] In the Door Range
  (if (== OtherActor (`GameplayStatics.GetPlayerCharacter` 0))
    (if (`self.isOpen`)
      _
      (elif (`self.Check 1`)
        (if (`self.Check 2`)
          (if (not (`self.Check 3`))
            (`KismetSystemLibrary.PrintString` "You need to active all nodes" :!label _label_2))
          (else
            (goto _label_2)))
        (else
          (goto _label_2))))))

(event `self.collision 1.OnComponentBeginOverlap`
  (params (OverlappedComponent :type "PrimitiveComponent Object Reference") (OtherActor :type "Actor Object Reference") (OtherComp :type "PrimitiveComponent Object Reference") (OtherBodyIndex :type Integer) (bFromSweep :type Boolean) (SweepResult :type "HitResult Structure (by ref)"))
  ;[1 1 1] Step 1
  (if (== OtherActor (`GameplayStatics.GetPlayerCharacter` 0))
    (if (not (`self.Check 1`))
      (`PrimitiveComponent.SetMaterial` (`self.Step 1`) 0 (`self.M_Open`))
      (`PrimitiveComponent.SetMaterial` (`self.Light 1`) 0 (`self.M_Open`))
      (bind _result (`/Engine/EditorBlueprintResources/StandardMacros.IncrementFloat` (`self.Count`))
        (:`  `
          (set `self.Count` _result)
          (set `self.Check 1` true))))))

(event `self.collision 2.OnComponentBeginOverlap`
  (params (OverlappedComponent :type "PrimitiveComponent Object Reference") (OtherActor :type "Actor Object Reference") (OtherComp :type "PrimitiveComponent Object Reference") (OtherBodyIndex :type Integer) (bFromSweep :type Boolean) (SweepResult :type "HitResult Structure (by ref)"))
  ;[1 1 1] Step 2
  (if (== OtherActor (`GameplayStatics.GetPlayerCharacter` 0))
    (if (not (`self.Check 2`))
      (`PrimitiveComponent.SetMaterial` (`self.Step 2`) 0 (`self.M_Open`))
      (`PrimitiveComponent.SetMaterial` (`self.Light 2`) 0 (`self.M_Open`))
      (bind _result (`/Engine/EditorBlueprintResources/StandardMacros.IncrementFloat` (`self.Count`))
        (:`  `
          (set `self.Count` _result)
          (set `self.Check 2` true))))))

(event `self.DoorInteraction.OnComponentEndOverlap`
  (params (OverlappedComponent :type "PrimitiveComponent Object Reference") (OtherActor :type "Actor Object Reference") (OtherComp :type "PrimitiveComponent Object Reference") (OtherBodyIndex :type Integer))
  ;[1 1 1] Out Of The Door Range
  (if (== OtherActor (`GameplayStatics.GetPlayerCharacter` 0))
    (if (`self.isOpen`)
      (goto _label :!via `Reverse`))))

(event `self.collision 3.OnComponentBeginOverlap`
  (params (OverlappedComponent :type "PrimitiveComponent Object Reference") (OtherActor :type "Actor Object Reference") (OtherComp :type "PrimitiveComponent Object Reference") (OtherBodyIndex :type Integer) (bFromSweep :type Boolean) (SweepResult :type "HitResult Structure (by ref)"))
  ;[1 1 1] Step 3
  (if (== OtherActor (`GameplayStatics.GetPlayerCharacter` 0))
    (if (not (`self.Check 3`))
      (`PrimitiveComponent.SetMaterial` (`self.Step 3`) 0 (`self.M_Open`))
      (`PrimitiveComponent.SetMaterial` (`self.Light 3`) 0 (`self.M_Open`))
      (bind _result (`/Engine/EditorBlueprintResources/StandardMacros.IncrementFloat` (`self.Count`))
        (:`  `
          (set `self.Count` _result)
          (set `self.Check 3` true))))))

(fn `UserConstructionScript`)