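; BP_DoorA is a two-panel sliding door the player opens and closes by pressing Interact near its LockSwitch.
; LockSwitch overlap prints a prompt and enables interaction, with six uses before the door reports out of order.
; A FlipFlop alternately plays and reverses a timeline that lerps DLeft and DRight along relative Y from their start positions.
; IsMoving blocks input during opening but is not set during closing.
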(event `self.ReceiveBeginPlay`
  ;[1 1 1] Start
  (`self.EnableInput` (`GameplayStatics.GetPlayerController` 0))
  (set `self.LeftStartLocation` (`SceneComponent.RelativeLocation` (`self.D_Left`)))
  (set `self.RightStartLocation` (`SceneComponent.RelativeLocation` (`self.D_Right`)))
  (set `self.InteractionCount` 6))

(event `self.LockSwitch.OnComponentBeginOverlap`
  (params (OverlappedComponent :type "PrimitiveComponent Object Reference") (OtherActor :type "Actor Object Reference") (OtherComp :type "PrimitiveComponent Object Reference") (OtherBodyIndex :type Integer) (bFromSweep :type Boolean) (SweepResult :type "HitResult Structure (by ref)"))
  ;[1 1 1] Close to the door
  (if (== OtherActor (`GameplayStatics.GetPlayerCharacter` 0))
    (if (> (`self.InteractionCount`) 0)
      (`KismetSystemLibrary.PrintString` "Press E to interact with the door." true false (struct :`R` 0.253365 :`G` 0.682292 :`B` 0.136768 :`A` 1.0) 3.0)
      (set `self.CanInteract` true)
      (else
        (`KismetSystemLibrary.PrintString` "The door is out of order. " true false (struct :`R` 0.376736 :`G` 0.116261 :`B` 0.338166 :`A` 1.0) 3.0)
        (set `self.CanInteract` false)))))

(event `self.LockSwitch.OnComponentEndOverlap`
  (params (OverlappedComponent :type "PrimitiveComponent Object Reference") (OtherActor :type "Actor Object Reference") (OtherComp :type "PrimitiveComponent Object Reference") (OtherBodyIndex :type Integer))
  ;[1 1 1] Far From the door
  (if (== OtherActor (`GameplayStatics.GetPlayerCharacter` 0))
    (set `self.CanInteract` false)))

(event `InputAction|Interact`
  (params (Key :type "Key Structure"))
  ;[1 1 1] Comment
  (:`Pressed`
    (if (not (`self.IsMoving`))
      (if (`self.CanInteract`)
        (if (> (`self.InteractionCount`) 0)
          (`/Engine/EditorBlueprintResources/StandardMacros.DecrementInt` (`self.InteractionCount`)
            (:`  `
              (`/Engine/EditorBlueprintResources/StandardMacros.FlipFlop`
                (:`A`
                  (set `self.IsMoving` true)
                  (bind (_direction _newtrack_0) (`Timeline|Timeline_0` :!label _label)
                    (:`Update`
                      (`SceneComponent.K2_SetRelativeLocation` (`self.D_Left`) (`KismetMathLibrary.VLerp` (`self.LeftStartLocation`) (`KismetMathLibrary.MakeVector` (.x (`self.LeftStartLocation`)) -115.0 (.z (`self.LeftStartLocation`))) _newtrack_0) false false)
                      (`SceneComponent.K2_SetRelativeLocation` (`self.D_Right`) (`KismetMathLibrary.VLerp` (`self.RightStartLocation`) (`KismetMathLibrary.MakeVector` (.x (`self.RightStartLocation`)) 120.0 (.z (`self.RightStartLocation`))) _newtrack_0) false false))
                    (:`Finished`
                      (set `self.IsMoving` false))))
                (:`B`
                  (goto _label :!via `Reverse`)))))
          (else
            (`KismetSystemLibrary.PrintString` "The door is out of order. " true false (struct :`R` 0.376736 :`G` 0.116261 :`B` 0.338166 :`A` 1.0) 3.0)))))))

(fn `UserConstructionScript`)